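; Leviathan's Wake runic attack actor that pushes physics-pushable targets in a line ahead of its instigator.
; On execute, it sphere-traces the Pawn profile along the instigator's forward direction at constant height, with debug drawing.
; Hit actors implementing BPI_PhysicsPushable receive a push message carrying that forward vector.
; It prints its name on BeginPlay and destroys itself shortly after the attack finishes.
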(event `self.ReceiveBeginPlay`
  (`KismetSystemLibrary.PrintString` "Leviathan's Wake!"))

(event `self.ExecuteRunicAttack`
  (bind _instigator (`self.Instigator`))
  (bind _returnvalue (`self.K2_GetActorLocation` _instigator))
  (bind (_returnvalue_x _returnvalue_y) (`KismetMathLibrary.BreakVector` (+ _returnvalue (* (`self.GetActorForwardVector` _instigator) (`self.m_MaxTravelDistance`)))))
  (bind _outhits (`KismetSystemLibrary.SphereTraceMultiByProfile` _returnvalue (`KismetMathLibrary.MakeVector` _returnvalue_x _returnvalue_y (.z _returnvalue)) (`self.m_SphereTraceRadius`) "Pawn" false (`|MakeArray` (`self.Instigator`) :!type "Actor Object Reference") "ForDuration"))
  (for _array_element _outhits
    (bind (_bblockinghit _binitialoverlap _time _distance _location _impactpoint _normal _impactnormal _physmat _hitactor) (`GameplayStatics.BreakHitResult` _array_element))
    (if (`KismetSystemLibrary.DoesImplementInterface` _hitactor "/Game/Gameplay/BPI_PhysicsPushable.BPI_PhysicsPushable_C")
      (message `/Game/Gameplay/BPI_PhysicsPushable.PhysicsPush` _hitactor (`self.GetActorForwardVector` (`self.GetInstigator`))))))

(event `self.FinishRunicAttack`
  (`KismetSystemLibrary.Delay` 0.2)
  (`self.K2_DestroyActor`))

(fn `UserConstructionScript`)