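; Leviathan's Wake runic attack actor: a projectile thrown along the instigator's forward vector that destroys itself after a timed delay.
; ExecuteRunicAttack enables sphere query collision, sets velocity and scales the particle effect.
; Each new overlapped actor other than the instigator triggers a camera shake, a physics push through BPI_PhysicsPushable if implemented, and a relayed hit.
; Global time dilation start and end events are defined but not called here.
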(event `self.ReceiveBeginPlay`
  (`KismetSystemLibrary.PrintString` "Leviathan's Wake!")
  (`PrimitiveComponent.SetCollisionEnabled` (`self.Sphere`) "NoCollision"))

(event `self.ExecuteRunicAttack`
  ;[1 1 1] Runic Action!
  (`self.ThrowLeviathan`)
  (`KismetSystemLibrary.Delay` 4.0)
  (`self.FinishRunicAttack`))

(event `ThrowLeviathan`
  ;[1 1 1] Runic Action!
  (`self.HandleThrow`))

(event `self.Sphere.OnComponentBeginOverlap`
  (params (OverlappedComponent :type "PrimitiveComponent Object Reference") (OtherActor :type "Actor Object Reference") (OtherComp :type "PrimitiveComponent Object Reference") (OtherBodyIndex :type Integer) (bFromSweep :type Boolean) (SweepResult :type "HitResult Structure (by ref)"))
  ;[1 1 1] Runic Action!
  (bind _returnvalue (`self.IsHitValidTarget` OtherActor))
  (if _returnvalue
    (`self.CameraShake`)
    (`self.HandleHit` OtherActor)))

(event `self.FinishRunicAttack`
  ;[1 1 1] Runic Action!
  (`KismetSystemLibrary.Delay` 0.2)
  (`self.K2_DestroyActor`))

(event `self.StartTimeDilation`
  ;[1 1 1] Time Dilation
  (`GameplayStatics.SetGlobalTimeDilation` (`self.m_RunicTimeDilation`)))

(event `self.EndTimeDilation`
  ;[1 1 1] Time Dilation
  (`GameplayStatics.SetGlobalTimeDilation` (`self.m_CachedTimeDilation`)))

(event `self.CameraShake`
  (`GameplayStatics.PlayWorldCameraShake` (`self.m_CameraShake`) (`self.K2_GetActorLocation` (`self.Instigator`)) 0.0 20000.0 0.0))

(fn `HandleHit`
  (params (i_HitActor :type "Actor Object Reference"))
  (if (`KismetSystemLibrary.DoesImplementInterface` i_HitActor "/Game/Gameplay/BPI_PhysicsPushable.BPI_PhysicsPushable_C")
    (message `/Game/Gameplay/BPI_PhysicsPushable.PhysicsPush` i_HitActor (`KismetMathLibrary.Normal` (`MovementComponent.Velocity` (`self.ProjectileMovement`)))))
  (`self.RelayHitInstance` i_HitActor)
  (`KismetArrayLibrary.Array_Add` (`self.m_HitRecordedActors`) i_HitActor)
  (`KismetSystemLibrary.PrintString` (`KismetSystemLibrary.GetDisplayName` i_HitActor)))

(fn `HandleThrow`
  (bind _m_vfxthrowscalemultiplier (`self.m_VFXThrowScaleMultiplier`))
  (`PrimitiveComponent.SetCollisionEnabled` (`self.Sphere`) "QueryOnly")
  (set `MovementComponent.Velocity` (* (`self.GetActorForwardVector` (`self.Instigator`)) (`self.m_ThrowVelocityMagnitude`)) (`self.ProjectileMovement`))
  (`SceneComponent.SetRelativeScale3D` (`self.ParticleSystem`) (`KismetMathLibrary.MakeVector` _m_vfxthrowscalemultiplier _m_vfxthrowscalemultiplier _m_vfxthrowscalemultiplier)))

(fn `IsHitValidTarget`
  (params (i_HitActor :type "Actor Object Reference (by ref)"))
  (returns (ReturnValue :type Boolean))
  (return (and (!= i_HitActor (`self.Instigator`)) (not (`KismetArrayLibrary.Array_Contains` (`self.m_HitRecordedActors`) i_HitActor)))))

(fn `UserConstructionScript`)