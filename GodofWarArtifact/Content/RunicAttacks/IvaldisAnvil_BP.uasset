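; Ivaldi's Anvil runic attack actor that deals frost damage to actors in a sphere around it.
; The sphere's collision stays off until ExecuteRunicAttack enables queries, then sends frost damage to each overlapping actor except the instigator and relays the hit.
; Separate events set and restore global time dilation and play a camera shake centered on the instigator.
; FinishRunicAttack destroys the actor after a short delay.
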(event `self.ReceiveBeginPlay`
  (`KismetSystemLibrary.PrintString` "Ivaldi's Anvil!")
  (`PrimitiveComponent.SetCollisionEnabled` (`self.Sphere`) "NoCollision"))

(event `CastAbility`)

(event `self.ExecuteRunicAttack`
  (`PrimitiveComponent.SetCollisionEnabled` (`self.Sphere`) "QueryOnly")
  (for _array_element (`PrimitiveComponent.GetOverlappingActors` (`self.Sphere`) null)
    (if (!= _array_element (`self.Instigator`))
      (`KismetSystemLibrary.PrintString` (`KismetSystemLibrary.GetDisplayName` _array_element))
      (message `/Game/Gameplay/BPI_Frost.FrostDamage` _array_element (`self.m_FrostDamage`))
      (`self.RelayHitInstance` _array_element))))

(event `self.FinishRunicAttack`
  (`KismetSystemLibrary.Delay` 0.2)
  (`self.K2_DestroyActor`))

(event `self.StartTimeDilation`
  (set `self.m_CachedTimeDilation` (`GameplayStatics.GetGlobalTimeDilation`))
  (`GameplayStatics.SetGlobalTimeDilation` (`self.m_RunicTimeDilation`)))

(event `self.EndTimeDilation`
  (`GameplayStatics.SetGlobalTimeDilation` (`self.m_CachedTimeDilation`)))

(event `self.CameraShake`
  (`GameplayStatics.PlayWorldCameraShake` (`self.m_CameraShake`) (`self.K2_GetActorLocation` (`self.Instigator`)) 0.0 20000.0 0.0))

(fn `UserConstructionScript`)