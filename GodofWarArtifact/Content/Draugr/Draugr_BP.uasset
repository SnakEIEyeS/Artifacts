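; Draugr enemy character Blueprint that reacts to hits, physics pushes and accumulated frost damage.
; Hit events play a montage looked up by reaction type; pushes apply a scaled velocity-change impulse to CharacterMovement.
; Frost past a threshold starts a delayed Freeze, which slows the AnimBP play rate and swaps in frozen materials.
; A second timer breaks the freeze, restoring play rate and the materials cached at BeginPlay; accumulated frost is never reset.
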(event `self.ReceiveBeginPlay`
  (`self.CacheOriginalMaterial`))

(event `/Game/Gameplay/BPI_CombatInfo.HitInstanceEvent`
  (params (i_HitInfo :type "/Game/Gameplay/HitInfoStruct Structure"))
  (`AnimInstance.Montage_Play` (`SkeletalMeshComponent.GetAnimInstance` (`self.Mesh`)) (`BlueprintMapLibrary.Map_Find` (`self.HitReactions`) i_HitInfo_m_ReactionTypeExpected_10_3229A45B48A1ED46D090ADBAEEC788D3) 1.0 "MontageLength" 0.0 true))

(event `/Game/Gameplay/BPI_Frost.FrostDamage`
  (params (i_FrostDamage :type "Float (single-precision)"))
  (bind _output_get (set `self.m_FrostDamage` (+ i_FrostDamage (`self.m_FrostDamage`))))
  (if (>= _output_get (`self.FreezeThreshold`))
    (`KismetSystemLibrary.K2_SetTimer` null "Freeze" (`self.m_FrostSetInTime`))))

(event `/Game/Gameplay/BPI_PhysicsPushable.PhysicsPush`
  (params (i_ForceDirection :type "Vector Structure"))
  (`CharacterMovementComponent.AddImpulse` (`self.CharacterMovement`) (* i_ForceDirection 10000.0) true))

(fn `BreakFreeze`
  (bind _asthird_person_anim_bp (cast `/Game/Mannequin/Animations/ThirdPerson_AnimBP` (`SkeletalMeshComponent.GetAnimInstance` (`self.Mesh`)))
    (:`then`
      (`/Game/Mannequin/Animations/ThirdPerson_AnimBP.ResetPlayRate` _asthird_person_anim_bp))
    (:`CastFailed`
      _))
  (`self.ChangeToOriginalMaterial`))

(fn `CacheOriginalMaterial`
  (set `self.m_OriginalBodyMaterial` (`PrimitiveComponent.GetMaterial` (`self.Mesh`) 0))
  (set `self.m_OriginalChestLogo` (`PrimitiveComponent.GetMaterial` (`self.Mesh`) 1)))

(fn `ChangeToFrozenMaterial`
  (`PrimitiveComponent.SetMaterial` (`self.Mesh`) 0 (`self.m_FreezeBodyMaterial`))
  (`PrimitiveComponent.SetMaterial` (`self.Mesh`) 1 (`self.m_FreezeChestLogo`)))

(fn `ChangeToOriginalMaterial`
  (`PrimitiveComponent.SetMaterial` (`self.Mesh`) 0 (`self.m_OriginalBodyMaterial`))
  (`PrimitiveComponent.SetMaterial` (`self.Mesh`) 1 (`self.m_OriginalChestLogo`)))

(fn `Freeze`
  (bind _asthird_person_anim_bp (cast `/Game/Mannequin/Animations/ThirdPerson_AnimBP` (`SkeletalMeshComponent.GetAnimInstance` (`self.Mesh`)))
    (:`then`
      (`/Game/Mannequin/Animations/ThirdPerson_AnimBP.FrozenPlayRate` _asthird_person_anim_bp (`self.m_FrostAnimPlayRate`)))
    (:`CastFailed`
      _))
  (`KismetSystemLibrary.K2_SetTimer` null "BreakFreeze" (`self.m_MaxFreezeTime`))
  (`self.ChangeToFrozenMaterial`))

(fn `UserConstructionScript`)