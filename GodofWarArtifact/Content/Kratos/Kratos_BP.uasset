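; Kratos player Blueprint that triggers light and heavy runic attacks from input.
; Each input action spawns its matching runic attack actor at Kratos's location and rotation, sets Kratos as its Instigator, then calls ExecuteRunicAttack on it.
; The attack behavior lives in the spawned actors, so this Blueprint only handles input and spawning.
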(event `InputAction|LightRunicAttack`
  (params (Key :type "Key Structure"))
  (bind (_returnvalue_location _returnvalue_rotation) (`KismetMathLibrary.BreakTransform` (`self.GetTransform`)))
  (:`Pressed`
    (bind _returnvalue (`|SpawnActorFromClass` (`self.LightRunicAttack`) (`KismetMathLibrary.MakeTransform` _returnvalue_location _returnvalue_rotation) "Undefined" "OverrideRootScale" null null))
    (set `Actor.Instigator` self _returnvalue)
    (`/Game/RunicAttacks/RunicAttack_BP.ExecuteRunicAttack` _returnvalue)))

(event `InputAction|HeavyRunicAttack`
  (params (Key :type "Key Structure"))
  (bind (_returnvalue_location _returnvalue_rotation) (`KismetMathLibrary.BreakTransform` (`self.GetTransform`)))
  (:`Pressed`
    (bind _returnvalue (`|SpawnActorFromClass` (`self.HeavyRunicAttack`) (`KismetMathLibrary.MakeTransform` _returnvalue_location _returnvalue_rotation) "Undefined" "OverrideRootScale" null null))
    (set `Actor.Instigator` self _returnvalue)
    (`/Game/RunicAttacks/RunicAttack_BP.ExecuteRunicAttack` _returnvalue)))

(fn `UserConstructionScript`)